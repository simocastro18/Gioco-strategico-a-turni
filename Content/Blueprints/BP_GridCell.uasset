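; BP_GridCell is a selectable grid cell that tints its mesh by its world height.
; BeginPlay creates a dynamic material and picks one of five banded colors from the actor's Z.
; Cursor hover toggles a highlight on unselected cells.
; Clicking hides every cell's highlight, then shows its own in magenta and sets IsSelected, which stays set because the reset node is unconnected.
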(event OnBeginCursorOver(StaticMesh)
  (params (TouchedComponent :type Primitive%20Component%20Object%20Reference))
  (if (not (Variables|Default|GetbIsSelected))
    (Development|PrintString "Touched")
    (Rendering|SetVisibility (Variables|Components|GetHoverHighlight) true false)))

(event OnEndCursorOver(StaticMesh)
  (params (TouchedComponent :type Primitive%20Component%20Object%20Reference))
  (if (not (Variables|Default|GetbIsSelected))
    (Rendering|SetVisibility (Variables|Components|GetHoverHighlight) false false)))

(event OnClicked(StaticMesh)
  (params (TouchedComponent :type Primitive%20Component%20Object%20Reference) (ButtonPressed :type Key%20Structure :default "None"))
  (bind _hoverhighlight (Variables|Components|GetHoverHighlight))
  (bind _outactors (Actor|GetAllActorsOfClass "BP_GridCell_C"))
  (for _array_element _outactors
    (Rendering|SetVisibility (Variables|BP_GridCell_C|GetHoverHighlight _array_element) false false))
  (Rendering|SetVisibility _hoverhighlight true false)
  (Rendering|Material|SetVectorParameterValueonMaterials _hoverhighlight "Color" "1.000000,0.000000,1.000000")
  (Variables|Default|SetbIsSelected true))

(event EventBeginPlay
  (bind _returnvalue (Rendering|Material|CreateDynamicMaterialInstance (Variables|Components|GetStaticMesh) 0 "/Game/Materials/M_CellColor.M_CellColor" "None" :!class /Script/Engine.PrimitiveComponent))
  (Rendering|Material|SetVectorParameterValue _returnvalue "Color" (Utilities|Select :Index (Math|Integer|Clamp(Integer) (Math|Float|Truncate (/ (.z (Transformation|GetActorLocation)) 5e+01)) 0 4) :Option%200 "(R=0.000000,G=0.000000,B=1.000000,A=1.000000)" :Option%201 "(R=0.000000,G=1.000000,B=0.000000,A=1.000000)" :Option%202 "(R=1.000000,G=1.000000,B=0.000000,A=1.000000)" :Option%203 "(R=2.000000,G=0.500000,B=0.000000,A=1.000000)" :Option%204 "(R=1.000000,G=0.000000,B=0.000000,A=1.000000)") :!class /Script/Engine.MaterialInstanceDynamic))

(event Collision|EventActorBeginOverlap
  (params (OtherActor :type Actor%20Object%20Reference)))

(event EventTick
  (params (DeltaSeconds :type Float%20%28single-precision%29)))

(fn ConstructionScript)